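; BP_Fire is a fire hazard that damages the player and sets them burning.
; Entering the collider passes a DoOnce that plays a sound, applies initial damage and sets the burning flag and death message on player pawn 0, regardless of the overlapping actor.
; A looping one-second timer applies tick damage while the player burns.
; Leaving re-arms the DoOnce and clears burning after a two-second delay.
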(event `self.ReceiveBeginPlay`
  ; Set Timer for Ticking Damage
  (`KismetSystemLibrary.K2_SetTimerDelegate` (delegate `TickingDamage`) 1.0 true))

(event `TickingDamage`
  (bind _collidingplayer (`self.CollidingPlayer`))
  ; Ticking Damage
  (if (!= null _collidingplayer)
    (if (`/Game/FirstPerson/Blueprints/BP_FirstPersonCharacter.isBurning` _collidingplayer)
      (`/Game/FirstPerson/Blueprints/BP_FirstPersonCharacter.damageHealth` _collidingplayer (`self.TickFireDamage`)))))

(event `self.Collider.OnComponentEndOverlap`
  (params (OverlappedComponent :type "PrimitiveComponent Object Reference") (OtherActor :type "Actor Object Reference") (OtherComp :type "PrimitiveComponent Object Reference") (OtherBodyIndex :type Integer))
  ; When Player Leaves Area
  (`|ExecutionSequence`
    (:`then_0`
      (`KismetSystemLibrary.Delay` 2.0)
      (set `/Game/FirstPerson/Blueprints/BP_FirstPersonCharacter.isBurning` false (`self.CollidingPlayer`)))
    (:`then_1`
      (goto _label :!via `Reset`))))

(event `self.Collider.OnComponentBeginOverlap`
  (params (OverlappedComponent :type "PrimitiveComponent Object Reference") (OtherActor :type "Actor Object Reference") (OtherComp :type "PrimitiveComponent Object Reference") (OtherBodyIndex :type Integer) (bFromSweep :type Boolean) (SweepResult :type "HitResult Structure (by ref)"))
  ;[1 1 1] Playing Sound and Damaging the Player
  (`/Engine/EditorBlueprintResources/StandardMacros.DoOnce` false :!label _label
    (:`Completed`
      (`GameplayStatics.PlaySoundAtLocation` "/Game/StarterContent/Audio/Collapse01.Collapse01" (`self.K2_GetActorLocation`) (struct) 1.0 1.0 0.0 null null null null)
      (bind _asbp_first_person_character (cast `/Game/FirstPerson/Blueprints/BP_FirstPersonCharacter` (`GameplayStatics.GetPlayerPawn` 0)))
      (bind _output_get (set `self.CollidingPlayer` _asbp_first_person_character))
      (`/Game/FirstPerson/Blueprints/BP_FirstPersonCharacter.damageHealth` _output_get (`self.FireDamage`))
      (set `/Game/FirstPerson/Blueprints/BP_FirstPersonCharacter.isBurning` true _output_get)
      (set `/Game/FirstPerson/Blueprints/BP_FirstPersonCharacter.DeathReason` "Next time, watch the fire!" _output_get))))

(fn `UserConstructionScript`)