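; BP_BasicDoor is an interactable door actor that the player opens and closes by pressing E while inside its collision volume.
; Overlap begin and end toggle input on player controller 0 and the billboard's visibility.
; E calls OpenCloseDoor, where a FlipFlop alternates playing and reversing a timeline that drives the door's yaw.
; Each timeline update also plays a 2D sound and hides the billboard.
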(event `OpenCloseDoor`
  ;[1 1 1] Open/Close Door Custom Event
  (`/Engine/EditorBlueprintResources/StandardMacros.FlipFlop`
    (:`A`
      (bind (_direction _dooropen) (`Timeline|Door_OpenClose` :!label _label)
        (:`Update`
          (`SceneComponent.K2_SetRelativeRotation` (`self.Door`) (`KismetMathLibrary.MakeRotator` 0.0 0.0 _dooropen) false false)
          (`GameplayStatics.PlaySound2D` (`self.AudioEffect`) 1.0 1.0 0.0 null null)
          (`SceneComponent.SetVisibility` (`self.Billboard`) false false))))
    (:`B`
      (goto _label :!via `Reverse`))))

(event `self.Collision.OnComponentBeginOverlap`
  (params (OverlappedComponent :type "PrimitiveComponent Object Reference") (OtherActor :type "Actor Object Reference") (OtherComp :type "PrimitiveComponent Object Reference") (OtherBodyIndex :type Integer) (bFromSweep :type Boolean) (SweepResult :type "HitResult Structure (by ref)"))
  ;[1 1 1] Enabling and Disabling Input on Collision
  (`self.EnableInput` (`GameplayStatics.GetPlayerController` 0))
  (`SceneComponent.SetVisibility` (`self.Billboard`) true false))

(event `self.Collision.OnComponentEndOverlap`
  (params (OverlappedComponent :type "PrimitiveComponent Object Reference") (OtherActor :type "Actor Object Reference") (OtherComp :type "PrimitiveComponent Object Reference") (OtherBodyIndex :type Integer))
  ;[1 1 1] Enabling and Disabling Input on Collision
  (`self.DisableInput` (`GameplayStatics.GetPlayerController` 0))
  (`SceneComponent.SetVisibility` (`self.Billboard`) false false))

(event `Key|E`
  (params (Key :type "Key Structure"))
  ;[1 1 1] Press E to Open/Close Door
  (:`Pressed`
    (`self.OpenCloseDoor`)))

(fn `UserConstructionScript`)