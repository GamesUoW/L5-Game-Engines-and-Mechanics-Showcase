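; BP_Button is an interactable button that toggles a spotlight when E is pressed near it.
; Overlapping ButtonCollider enables input for player 0 and ending the overlap disables it, with no check on which actor overlaps.
; Each press flips the SpotLight intensity, starting with off, and calls InteractButton.
; InteractButton uses its own FlipFlop to play or reverse a Timeline that slides the button along its relative X axis.
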(event `self.Button Collider.OnComponentBeginOverlap`
  (params (OverlappedComponent :type "PrimitiveComponent Object Reference") (OtherActor :type "Actor Object Reference") (OtherComp :type "PrimitiveComponent Object Reference") (OtherBodyIndex :type Integer) (bFromSweep :type Boolean) (SweepResult :type "HitResult Structure (by ref)"))
  ;[1 1 1] Enable/Disable Input
  (`self.EnableInput` (`GameplayStatics.GetPlayerController` 0)))

(event `self.Button Collider.OnComponentEndOverlap`
  (params (OverlappedComponent :type "PrimitiveComponent Object Reference") (OtherActor :type "Actor Object Reference") (OtherComp :type "PrimitiveComponent Object Reference") (OtherBodyIndex :type Integer))
  ;[1 1 1] Enable/Disable Input
  (`self.DisableInput` (`GameplayStatics.GetPlayerController` 0)))

(event `Key|E`
  (params (Key :type "Key Structure"))
  (bind _spotlight (`self.SpotLight`))
  ;[1 1 1] Press E to Animate Button and Turn On/Off the light
  (:`Pressed`
    (`self.InteractButton`)
    (`/Engine/EditorBlueprintResources/StandardMacros.FlipFlop`
      (:`A`
        (`LightComponent.SetIntensity` _spotlight 0.0))
      (:`B`
        (`LightComponent.SetIntensity` _spotlight 5000.0)))))

(event `InteractButton`
  ;[1 1 1] Button Animation
  (`/Engine/EditorBlueprintResources/StandardMacros.FlipFlop`
    (:`A`
      (bind (_direction _button_press) (`Timeline|Timeline` :!label _label)
        (:`Update`
          (`SceneComponent.K2_SetRelativeLocation` (`self.Button`) (`KismetMathLibrary.MakeVector` _button_press) false false))))
    (:`B`
      (goto _label :!via `Reverse`))))

(fn `UserConstructionScript`)