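; BP_SwingingBlades is a swinging axe hazard that hurts the player on contact.
; On BeginPlay, the Swinging_Motion timeline starts and drives the axe mesh's relative pitch.
; When the Collider overlaps the player pawn, it casts to BP_FirstPersonCharacter, applies Damage, sets a custom death reason and runs the character's death check.
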(event `self.ReceiveBeginPlay`
  (`self.SwingBlades`))

(event `self.Collider.OnComponentBeginOverlap`
  (params (OverlappedComponent :type "PrimitiveComponent Object Reference") (OtherActor :type "Actor Object Reference") (OtherComp :type "PrimitiveComponent Object Reference") (OtherBodyIndex :type Integer) (bFromSweep :type Boolean) (SweepResult :type "HitResult Structure (by ref)"))
  (if (== OtherActor (`GameplayStatics.GetPlayerPawn` 0))
    (bind _asbp_first_person_character (cast `/Game/FirstPerson/Blueprints/BP_FirstPersonCharacter` OtherActor))
    (`/Game/FirstPerson/Blueprints/BP_FirstPersonCharacter.damageHealth` _asbp_first_person_character (`self.Damage`))
    (set `/Game/FirstPerson/Blueprints/BP_FirstPersonCharacter.DeathReason` "You went out swinging!" _asbp_first_person_character)
    (`/Game/FirstPerson/Blueprints/BP_FirstPersonCharacter.CheckDeath` _asbp_first_person_character)))

(event `SwingBlades`
  (bind (_direction _swinging1) (`Timeline|Swinging_Motion`)
    (:`Update`
      (`SceneComponent.K2_SetRelativeRotation` (`self.Axe_Mesh`) (`KismetMathLibrary.MakeRotator` 0.0 _swinging1) false false))))

(fn `UserConstructionScript`)